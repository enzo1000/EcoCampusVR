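; BP_Button is a VR push button that triggers Launch on every Poubelle_Blueprint actor in the level.
; VRPawn overlap with its Box moves the Button component down, and end overlap returns it to the position saved at BeginPlay.
; Tick polls the button's relative Z and, while it is below a fixed threshold, gathers all those actors and calls Launch every frame, rather than once per press.
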(event `self.ReceiveTick`
  (params (DeltaSeconds :type "Float (single-precision)"))
  (bind (_relativelocation_x _relativelocation_y _relativelocation_z) (`KismetMathLibrary.BreakVector` (`SceneComponent.RelativeLocation` (`self.Button`))))
  (if (< _relativelocation_z 1.0)
    (bind _outactors (`GameplayStatics.GetAllActorsOfClass` "/Game/EcoCampus/Poubelles/Poubelle_Blueprint.Poubelle_Blueprint_C"))
    (for _array_element _outactors
      (`/Game/EcoCampus/Poubelles/Poubelle_Blueprint.Launch` _array_element))))

(event `self.ReceiveBeginPlay`
  (set `self.ButtonStart` (`SceneComponent.RelativeLocation` (`self.Button`))))

(event `self.Box.OnComponentBeginOverlap`
  (params (OverlappedComponent :type "PrimitiveComponent Object Reference") (OtherActor :type "Actor Object Reference") (OtherComp :type "PrimitiveComponent Object Reference") (OtherBodyIndex :type Integer) (bFromSweep :type Boolean) (SweepResult :type "HitResult Structure (by ref)"))
  (cast `/Game/VRTemplate/Blueprints/VRPawn` OtherActor)
  (`KismetSystemLibrary.MoveComponentTo` (`self.Button`) (- (`self.ButtonStart`) (0.0 0.0 5.0))))

(event `self.Box.OnComponentEndOverlap`
  (params (OverlappedComponent :type "PrimitiveComponent Object Reference") (OtherActor :type "Actor Object Reference") (OtherComp :type "PrimitiveComponent Object Reference") (OtherBodyIndex :type Integer))
  (cast `/Game/VRTemplate/Blueprints/VRPawn` OtherActor)
  (`KismetSystemLibrary.MoveComponentTo` (`self.Button`) (`self.ButtonStart`)))

(fn `UserConstructionScript`)